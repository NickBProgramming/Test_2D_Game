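; LevelExit is a trigger volume that moves the player to another level, named by LevelName.
; When the player character overlaps its Box, it stores SpawnID on the game instance through a SetSpawnID helper, then opens the level by name.
; If that helper fails, it prints a cast failure message instead of travelling.
; The construction script sizes the box from the BoxExtent variable.
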(event `self.Box.OnComponentBeginOverlap`
  (params (OverlappedComponent :type "PrimitiveComponent Object Reference") (OtherActor :type "Actor Object Reference") (OtherComp :type "PrimitiveComponent Object Reference") (OtherBodyIndex :type Integer) (bFromSweep :type Boolean) (SweepResult :type "HitResult Structure (by ref)"))
  (if (== OtherActor (`GameplayStatics.GetPlayerCharacter` 0))
    (bind _success (`/Game/Gamemode/FL_SpawnIDs.SetSpawnID` (`GameplayStatics.GetGameInstance`) (`self.Spawn ID`)))
    (if _success
      (`GameplayStatics.OpenLevel` (`self.LevelName`))
      (else
        (`KismetSystemLibrary.PrintString` "Function Library instance cast failed" true true (struct :`R` 1.0 :`B` 0.029831 :`A` 1.0) 10.0)))))

(fn `UserConstructionScript`
  (`BoxComponent.SetBoxExtent` (`self.Box`) (`self.Box_Extent`) true))