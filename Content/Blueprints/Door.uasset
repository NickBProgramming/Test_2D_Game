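; Sliding 2D door that opens by player proximity or through an Interaction event, moving its PaperSprite along relative X.
; Box1 overlaps with Player_Character set Open and, unless IsSwitch is set, play or reverse the OpenClose timeline.
; Interaction toggles IsOpen and drives a separate OpenCloseInput timeline, regardless of IsSwitch.
; Construction script applies BoxExtent and sets PlayRate on OpenClose only; a delayed hide/show chain is left unconnected.
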(event `self.Box1.OnComponentBeginOverlap`
  (params (OverlappedComponent :type "PrimitiveComponent Object Reference") (OtherActor :type "Actor Object Reference") (OtherComp :type "PrimitiveComponent Object Reference") (OtherBodyIndex :type Integer) (bFromSweep :type Boolean) (SweepResult :type "HitResult Structure (by ref)"))
  (bind _papersprite (`self.PaperSprite`))
  (cast `/Game/Character/Player_Character` OtherActor)
  (set `self.Open` true)
  (if (not (`self.isSwitch`))
    (bind (_direction _location) (`Timeline|Open/Close` :!label _label)
      (:`Update`
        (`SceneComponent.K2_SetRelativeLocation` _papersprite (`KismetMathLibrary.MakeVector` _location (.y (`SceneComponent.RelativeLocation` _papersprite)) (.z (`SceneComponent.RelativeLocation` _papersprite))) false false)))))

(event `self.Box1.OnComponentEndOverlap`
  (params (OverlappedComponent :type "PrimitiveComponent Object Reference") (OtherActor :type "Actor Object Reference") (OtherComp :type "PrimitiveComponent Object Reference") (OtherBodyIndex :type Integer))
  (cast `/Game/Character/Player_Character` OtherActor)
  (set `self.Open` false)
  (if (not (`self.isSwitch`))
    (goto _label :!via `Reverse`)))

(event `/Game/Blueprints/IF_Interaction.Interaction`
  (bind _papersprite (`self.PaperSprite`))
  (if (not (`self.isOpen`))
    (set `self.isOpen` true)
    (bind (_direction _location) (`Timeline|Open/Close Input` :!label _label_2)
      (:`Update`
        (`SceneComponent.K2_SetRelativeLocation` _papersprite (`KismetMathLibrary.MakeVector` _location (.y (`SceneComponent.RelativeLocation` _papersprite)) (.z (`SceneComponent.RelativeLocation` _papersprite))) false false)))
    (else
      (set `self.isOpen` false)
      (goto _label_2 :!via `Reverse`))))

(fn `UserConstructionScript`
  (`BoxComponent.SetBoxExtent` (`self.Box1`) (`self.Box Extent`) true)
  (`TimelineComponent.SetPlayRate` (`self.Open/Close`) (`self.Play Rate`)))